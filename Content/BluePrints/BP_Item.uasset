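; BP_Item is an item Blueprint that gives itself a random name and prints it.
; The Construction Script replaces the default "unamedItem" name with a pick from three hard-coded names, then prints it with "is holding" appended.
; The random index range includes the array length, so the pick can fall out of bounds.
; BeginPlay prints the name; overlap and Tick are unused.
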(event EventBeginPlay
  (Development|PrintString (Variables|Default|Getname)))

(event Collision|EventActorBeginOverlap
  (params (OtherActor :type Actor%20Object%20Reference)))

(event EventTick
  (params (DeltaSeconds :type Float%20%28single-precision%29)))

(fn ConstructionScript
  (bind _returnvalue (Utilities|String|MakeLiteralString "Bagert"))
  (bind _returnvalue_2 (Utilities|String|MakeLiteralString "Brian"))
  (bind _returnvalue_3 (Utilities|String|MakeLiteralString "Jaedon"))
  (bind _array (Utilities|Array|MakeArray _returnvalue_2 _returnvalue_3 _returnvalue))
  ;[1 1 1] see if the name has been changed
  (if (Utilities|Enum|Equal(Enum) (Variables|Default|Getname) "unamedItem")
    (Utilities|Array|Shuffle _array)
    (bind _output_get (Variables|Default|Setname (Utilities|Array|Get(acopy) _array (Math|Random|RandomIntegerinRange 0 (Utilities|Array|Length _array)))))
    (Development|PrintString (Utilities|String|Append _output_get " is holding") true true "(R=0.043863,G=1.000000,B=0.000000,A=1.000000)" 1e+01)))