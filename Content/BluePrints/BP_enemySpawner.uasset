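; BP_enemySpawner is a wave spawner that repopulates the level with BP_Enemy whenever none remain.
; On BeginPlay it gathers all BP_EnemySpawnLocation actors, prints their count for debugging, then spawns a first wave.
; Each wave rolls randomly per location, with roughly an 80% chance of spawning an enemy at that transform.
; A self-calling event with a Delay polls for living enemies every two seconds and triggers the next wave.
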(event Custom|SpawnEnemyes
  (for _array_element (stale EventBeginPlay _outactors)
    (if (> (Math|Random|RandomFloat) 0.2)
      (Game|SpawnActorfromClass "/Game/BluePrints/BP_Enemy.BP_Enemy_C" (Transformation|GetActorTransform _array_element) "Undefined" "MultiplyWithRoot" 0 0))))

(event Custom|Check%20enemy%20count
  (bind _outactors (Actor|GetAllActorsOfClass "/Game/BluePrints/BP_Enemy.BP_Enemy_C"))
  (if (> (Utilities|Array|Length _outactors) 0)
    _
    (else
      (CallFunction|SpawnEnemyes)))
  (Utilities|FlowControl|Delay 2.0)
  (CallFunction|CheckEnemyCount))

(event EventBeginPlay
  (bind _outactors (Actor|GetAllActorsOfClass "/Game/BluePrints/BP_EnemySpawnLocation.BP_EnemySpawnLocation_C"))
  (Development|PrintString (Utilities|String|Append "there are" (Utilities|String|ToString(Integer) (Utilities|Array|Length _outactors)) "spawners in the level") true true "(R=0.000000,G=0.660000,B=1.000000,A=1.000000)" 1e+01)
  (CallFunction|SpawnEnemyes)
  (CallFunction|CheckEnemyCount))

(fn ConstructionScript)