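; BP_Enemy is an enemy that takes damage when the player character overlaps its capsule, using the held item's GetDamage with the enemy's ElementalType.
; At zero health it swaps alive and dead billboards, plays a sound and destroys itself after a delay; IsDead is never set true.
; BeginPlay plays a randomly delayed spawn sound, checks for zero health, and randomly picks any unset name or team material from shuffled arrays.
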(event OnComponentBeginOverlap(Capsule)
  (params (OverlappedComponent :type Primitive%20Component%20Object%20Reference) (OtherActor :type Actor%20Object%20Reference) (OtherComp :type Primitive%20Component%20Object%20Reference) (OtherBodyIndex :type Integer) (bFromSweep :type Boolean) (SweepResult :type Hit%20Result%20Structure%20%28by%20ref%29))
  ;[1 1 1] if touching player take damage
  (bind _asbp_third_person_character (Utilities|Casting|CastToBP_ThirdPersonCharacter OtherActor))
  (bind _damage (Default|GetDamage (Variables|/Game/ThirdPerson/Blueprints/BP_ThirdPersonCharacter.BP_ThirdPersonCharacter_C|Gethelditem _asbp_third_person_character) (Variables|Default|GetelementalType)))
  (Development|PrintString (Utilities|String|Append "i took" (Utilities|String|ToString(Integer) _damage) " damage"))
  (bind _output_get (Variables|Default|SetHealth (- (Variables|Default|GetHealth) _damage)))
  (Development|PrintString (Utilities|String|Append "my health is now" (Utilities|String|ToString(Float) _output_get)))
  (CallFunction|ITOokDamage))

(event Custom|I%20TOok%20Damage
  ;[1 1 1] When i take damage, check health, check is still alive
  (if (<= (Variables|Default|GetHealth) 0.0)
    (if (not (Variables|Default|GetIs%20Dead))
      ;[1 1 1] Change billboard, play sound delay deleate
      (Variables|Default|SetIs%20Dead false)
      (Development|SetHiddeninGame (Variables|Default|GetBillAlive) true false)
      (Development|SetHiddeninGame (Variables|Default|GetBill_ADead) false false)
      (Audio|Components|Audio|Play (Variables|Default|GetPETA) 0.0)
      (Development|PrintString (Utilities|String|Append "you killed " (Utilities|String|ToString(Name) (Variables|Default|GetEnemyName)) "!"))
      (Utilities|FlowControl|Delay 1.0)
      (Actor|DestroyActor))))

(event EventBeginPlay
  (bind _materials (Variables|Default|GetMaterials))
  (bind _names (Variables|Default|GetNames))
  (Utilities|FlowControl|Sequence
    (:then_0
      ;[1 1 1] Set billboard and play spawn sound
      (Development|SetHiddeninGame (Variables|Default|GetBill_ADead) true false)
      (Utilities|FlowControl|Delay (Math|Random|RandomFloatinRange 0.1 1.0))
      (Audio|Components|Audio|Play (Variables|Default|Getpeter) 0.0)
      ;[1 1 1] See if i spawn with 0 health
      (Utilities|FlowControl|Delay 1.0)
      (CallFunction|ITOokDamage)
      ;[1 1 1] When i take damage, check health, check is still alive
      (if (<= (Variables|Default|GetHealth) 0.0)
        (if (not (Variables|Default|GetIs%20Dead))
          ;[1 1 1] Change billboard, play sound delay deleate
          (Variables|Default|SetIs%20Dead false)
          (Development|SetHiddeninGame (Variables|Default|GetBillAlive) true false)
          (Development|SetHiddeninGame (Variables|Default|GetBill_ADead) false false)
          (Audio|Components|Audio|Play (Variables|Default|GetPETA) 0.0)
          (Development|PrintString (Utilities|String|Append "you killed " (Utilities|String|ToString(Name) (Variables|Default|GetEnemyName)) "!"))
          (Utilities|FlowControl|Delay 1.0)
          (Actor|DestroyActor))))
    (:then_1
      (Utilities|Array|Shuffle (Variables|Default|GetNames)))
    (:then_2
      ;[1 1 1] Set material
      (Utilities|IsValid (Variables|Default|GetEnemyTeamMaterial)
        (:Is%20Valid
          (Development|PrintString "Alredy Existing Mateirial" true true "(R=1.000000,G=0.117262,B=0.000000,A=1.000000)"))
        (:Is%20Not%20Valid
          (Development|PrintString "Picking a new material" true true "(R=0.000000,G=1.000000,B=0.390325,A=1.000000)")
          (Utilities|Array|Shuffle _materials)
          (Variables|Default|SetEnemyTeamMaterial (Utilities|Array|Get(acopy) _materials))))
      (Rendering|Material|SetMaterial (Variables|Default|GetBillAlive) 0 (Variables|Default|GetEnemyTeamMaterial)))
    (:then_3
      ;[1 1 1] Set name
      (if (== (Variables|Default|GetEnemyName) "")
        (Development|PrintString "picking a new name" true true "(R=0.000000,G=1.000000,B=0.390325,A=1.000000)")
        (Utilities|Array|Shuffle _names)
        (bind _output_get (Variables|Default|SetEnemyName (Utilities|Array|Get(acopy) _names)))
        (else
          (Development|PrintString "Alredy Existing name" true true "(R=1.000000,G=0.117262,B=0.000000,A=1.000000)")))
      (Development|PrintString (Utilities|String|Append "my name is " (Utilities|String|ToString(Name) _output_get) "!")))))

(fn ConstructionScript)